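; BP_Bow is an archery bow Blueprint that measures how far its string grab point is pulled from its resting distance.
; BeginPlay caches the distance between Scene and SphereString as a baseline, along with the string sphere's relative location.
; Tick stores the current world-space distance minus that baseline in Distance.
; A debug print of Distance is left disconnected, and nothing here uses the saved location.
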(event `self.ReceiveBeginPlay`
  (set `self.DefaultDistanceBetweenGrabs` (`KismetMathLibrary.Vector_Distance` (`SceneComponent.K2_GetComponentLocation` (`self.Scene`)) (`SceneComponent.K2_GetComponentLocation` (`self.SphereString`))))
  (set `self.OriginalLocation` (`SceneComponent.RelativeLocation` (`self.SphereString`))))

(event `self.ReceiveTick`
  (params (DeltaSeconds :type "Float (single-precision)"))
  (bind _output_get (set `self.Distance` (- (`KismetMathLibrary.Vector_Distance` (`SceneComponent.K2_GetComponentLocation` (`self.Scene`)) (`SceneComponent.K2_GetComponentLocation` (`self.SphereString`))) (`self.DefaultDistanceBetweenGrabs`)))))

(fn `UserConstructionScript`)